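; Roof puzzle Blueprint where a lever lowers a hatch and clears fog.
; Pressing E runs a sphere trace at the player's capsule; hitting a "lever"-tagged component plays a lever-rotation timeline that calls CheckStatue every update.
; CheckStatue, gated by Opened and DoOnce, moves the hatch down and fades radial fog extinction through a second timeline.
; Setup of the player reference, Opened and initial fog is unconnected and never runs.
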(event `Key|E`
  (params (Key :type "Key Structure"))
  (bind _returnvalue (`SceneComponent.K2_GetComponentLocation` (`Character.CapsuleComponent` (`self.PlayerCharacter`))))
  ; Colision detection on key press using sphere trace
  (:`Pressed`
    (bind (_outhit _returnvalue_2) (`KismetSystemLibrary.SphereTraceSingle` :`Start` _returnvalue :`End` _returnvalue :`Radius` 200.0 :`TraceChannel` "TraceTypeQuery1" :`bIgnoreSelf` false))
    ; Checks to see if the colided object is the lever
    (if _returnvalue_2
      (if (`ActorComponent.ComponentHasTag` (`.HitComponent` (`GameplayStatics.BreakHitResult` _outhit)) "lever")
        ; Creates a timeline for the lever animation with max and min lever rotation in the lerp. The relative rotation is then passed the lerp. Finally, the function check statue is called.
        (bind (_direction _move) (`Timeline|Timeline` :!via `PlayFromStart`)
          (:`Update`
            (`SceneComponent.K2_SetRelativeRotation` (`self.Lever`) (`KismetMathLibrary.RLerp` (struct :`Pitch` 30.0) (struct :`Pitch` -40.0) _move) false false)
            (`self.CheckStatue`)))))))

(event `CheckStatue`
  (bind _hatch (`self.Hatch`))
  (bind (_returnvalue_x _returnvalue_y _returnvalue_z) (`KismetMathLibrary.BreakVector` (`SceneComponent.K2_GetComponentLocation` _hatch)))
  ; Puzzle completion is compaired to see what phase of the puzzle is being checked and will then run the current check values
  (if (<= (`.Value` (break `RigVMFunction_MathIntMake` (`self.Opened`))) 0)
    ; retrieves the current location and relative rotation and then moves the waterfall out of the level
    (`/Engine/EditorBlueprintResources/StandardMacros.DoOnce` false
      (:`Completed`
        (`KismetSystemLibrary.MoveComponentTo` (`self.Hatch`) (`KismetMathLibrary.MakeVector` _returnvalue_x _returnvalue_y (- _returnvalue_z 20.0)) (`SceneComponent.RelativeRotation` _hatch) false false 2.0)
        (set `self.Opened` (make `RigVMFunction_MathIntMake` 1))
        (bind (_direction _newtrack_0) (`Timeline|Timeline_0`)
          (:`Update`
            (`LocalFogVolumeComponent.SetRadialFogExtinction` (`self.Fog`) (`KismetMathLibrary.Lerp` 2.0 0.0 _newtrack_0))))))))

(fn `UserConstructionScript`)