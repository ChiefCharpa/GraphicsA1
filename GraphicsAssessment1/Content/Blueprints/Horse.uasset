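; Horse Blueprint that plays a reaction animation when Q is pressed near the player.
; On Q, a sphere trace around its Box component checks whether the hit component carries the Player tag.
; If so, the rigged horse mesh randomly plays either a head-move or a bow animation once.
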(event `Key|Q` :consume false
  (params (Key :type "Key Structure"))
  (bind _returnvalue (`SceneComponent.K2_GetComponentLocation` (`self.Box`)))
  (:`Pressed`
    (bind (_outhit _returnvalue_2) (`KismetSystemLibrary.SphereTraceSingle` :`Start` _returnvalue :`End` _returnvalue :`Radius` 300.0 :`TraceChannel` "TraceTypeQuery1" :`bIgnoreSelf` false))
    (if _returnvalue_2
      (if (`ActorComponent.ComponentHasTag` (`.HitComponent` (`GameplayStatics.BreakHitResult` _outhit)) "Player")
        (if (== (`KismetMathLibrary.RandomBool`) true)
          (`SkeletalMeshComponent.PlayAnimation` (`self.FullyRiggedHorsegood`) "/Game/Skel/FullyRiggedHorsegood_Anim_rig_movehead.FullyRiggedHorsegood_Anim_rig_movehead" false)
          (else
            (`SkeletalMeshComponent.PlayAnimation` (`self.FullyRiggedHorsegood`) "/Game/Skel/FullyRiggedHorsegood_Anim_Bow.FullyRiggedHorsegood_Anim_Bow" false)))))))

(fn `UserConstructionScript`)