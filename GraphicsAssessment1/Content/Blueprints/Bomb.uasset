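; Bomb actor for a two-step pick-up-and-plant demolition interaction on the F key.
; An integer-like Progress state gates sphere traces around the player, matching component tags to first collect the dynamite, then place it at the plant spot.
; A Timeline acts as the fuse; on finish it calls CETrigger on the child-actor FS_MasterField, hides the props and activates the explosion effect.
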(event `self.ReceiveBeginPlay`
  (`SceneComponent.SetVisibility` (`self.dynamite`) false false)
  (`SceneComponent.SetVisibility` (`self.PlantSpot`) true false)
  (`SceneComponent.SetVisibility` (`self.dynamite1`) true false)
  (bind _asfs_master_field (cast `/Engine/EditorResources/FieldNodes/FS_MasterField` (`ChildActorComponent.ChildActor` (`self.Force`))))
  (set `self.FS` _asfs_master_field)
  ; Initial setters and getters for the containers
  (bind _asbp_third_person_character (cast `/Game/ThirdPerson/Blueprints/BP_ThirdPersonCharacter` (`GameplayStatics.GetPlayerCharacter` 0)))
  (set `self.PlayerCharacter` _asbp_third_person_character)
  (set `self.Progress` 0))

(event `Key|F` :consume false
  (params (Key :type "Key Structure"))
  (bind _playercharacter (`self.PlayerCharacter`))
  (bind _playercharacter_2 (`self.PlayerCharacter`))
  (bind _returnvalue (`SceneComponent.K2_GetComponentLocation` (`Character.CapsuleComponent` _playercharacter)))
  (bind _returnvalue_2 (`SceneComponent.K2_GetComponentLocation` (`Character.CapsuleComponent` _playercharacter_2)))
  (:`Pressed`
    (if (<= (`self.Progress`) 0)
      ; Colision detection on key press using sphere trace
      (bind (_outhit _returnvalue_3) (`KismetSystemLibrary.SphereTraceSingle` _returnvalue_2 _returnvalue_2 200.0 "TraceTypeQuery1" true (`|MakeArray` _playercharacter_2 :!type "Actor Object Reference") "Persistent" false))
      ; Checks to see if the colided object is the lever
      (if _returnvalue_3
        (if (`ActorComponent.ComponentHasTag` (`.HitComponent` (`GameplayStatics.BreakHitResult` _outhit)) "Dyna1")
          (`SceneComponent.SetVisibility` (`self.dynamite1`) false false)
          (set `self.Progress` 1)))
      (elif (<= (`self.Progress`) 1)
        ; Colision detection on key press using sphere trace
        (bind (_outhit_2 _returnvalue_4) (`KismetSystemLibrary.SphereTraceSingle` _returnvalue _returnvalue 200.0 "TraceTypeQuery1" false (`|MakeArray` _playercharacter :!type "Actor Object Reference") "None" false))
        ; Checks to see if the colided object is the lever
        (if _returnvalue_4
          (if (`ActorComponent.ComponentHasTag` (`.HitComponent` (`GameplayStatics.BreakHitResult` _outhit_2)) "Plant")
            (`SceneComponent.SetVisibility` (`self.dynamite`) true false)
            (`Timeline|Timeline`
              (:`Finished`
                (`/Engine/EditorResources/FieldNodes/FS_MasterField.CE_Trigger` (`self.FS`))
                (`SceneComponent.SetVisibility` (`self.PlantSpot`) false false)
                (`SceneComponent.SetVisibility` (`self.dynamite`) false false)
                (`ActorComponent.Activate` (`self.Explosion`) false)
                (set `self.Progress` 2)))))))))

(fn `UserConstructionScript`)