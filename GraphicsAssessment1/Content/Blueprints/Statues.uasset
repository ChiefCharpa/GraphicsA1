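; Statue rotation puzzle Blueprint with three phases, opened by a lever.
; F sphere-traces around the player and, by component tag, turns one of six statues 90 degrees, gated by a DoOnce and delay.
; E on the lever plays a rotation timeline that calls CheckStatue on every update.
; CheckStatue exact-matches statue yaws for the current PuzzleCompletion phase, moving away two waterfalls in turn, then lowering the final door.
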(event `self.ReceiveBeginPlay`
  ; Initial setters and getters for the containers
  (bind _asbp_third_person_character (cast `/Game/ThirdPerson/Blueprints/BP_ThirdPersonCharacter` (`GameplayStatics.GetPlayerCharacter` 0)))
  (set `self.PlayerCharacter` _asbp_third_person_character)
  (set `self.PuzzleCompletion` (make `RigVMFunction_MathIntMake` 0)))

(event `Key|F`
  (params (Key :type "Key Structure"))
  (bind _statue1 (`self.Statue1`))
  (bind _statue2 (`self.Statue2`))
  (bind _statue3 (`self.Statue3`))
  (bind _statue5 (`self.Statue5`))
  (bind _statue6 (`self.Statue6`))
  (bind _statue4 (`self.Statue4`))
  (bind (_returnvalue_roll _returnvalue_pitch _returnvalue_yaw) (`KismetMathLibrary.BreakRotator` (`SceneComponent.K2_GetComponentRotation` _statue1)))
  (bind (_returnvalue_roll_2 _returnvalue_pitch_2 _returnvalue_yaw_2) (`KismetMathLibrary.BreakRotator` (`SceneComponent.K2_GetComponentRotation` _statue6)))
  (bind (_returnvalue_roll_3 _returnvalue_pitch_3 _returnvalue_yaw_3) (`KismetMathLibrary.BreakRotator` (`SceneComponent.K2_GetComponentRotation` _statue2)))
  (bind (_returnvalue_roll_4 _returnvalue_pitch_4 _returnvalue_yaw_4) (`KismetMathLibrary.BreakRotator` (`SceneComponent.K2_GetComponentRotation` _statue3)))
  (bind (_returnvalue_roll_5 _returnvalue_pitch_5 _returnvalue_yaw_5) (`KismetMathLibrary.BreakRotator` (`SceneComponent.K2_GetComponentRotation` _statue4)))
  (bind (_returnvalue_roll_6 _returnvalue_pitch_6 _returnvalue_yaw_6) (`KismetMathLibrary.BreakRotator` (`SceneComponent.K2_GetComponentRotation` _statue5)))
  (bind _returnvalue (`SceneComponent.K2_GetComponentLocation` (`Character.CapsuleComponent` (`self.PlayerCharacter`))))
  (bind (_returnvalue_roll_7 _returnvalue_pitch_7 _returnvalue_yaw_7) (`KismetMathLibrary.BreakRotator` (`KismetMathLibrary.MakeRotator` 0.0 0.0 (+ _returnvalue_yaw 90.0))))
  (bind (_returnvalue_roll_8 _returnvalue_pitch_8 _returnvalue_yaw_8) (`KismetMathLibrary.BreakRotator` (`KismetMathLibrary.MakeRotator` 0.0 0.0 (+ _returnvalue_yaw_3 90.0))))
  (bind (_returnvalue_roll_9 _returnvalue_pitch_9 _returnvalue_yaw_9) (`KismetMathLibrary.BreakRotator` (`KismetMathLibrary.MakeRotator` 0.0 0.0 (+ _returnvalue_yaw_2 90.0))))
  (bind (_returnvalue_roll_10 _returnvalue_pitch_10 _returnvalue_yaw_10) (`KismetMathLibrary.BreakRotator` (`KismetMathLibrary.MakeRotator` 0.0 0.0 (+ _returnvalue_yaw_4 90.0))))
  (bind (_returnvalue_roll_11 _returnvalue_pitch_11 _returnvalue_yaw_11) (`KismetMathLibrary.BreakRotator` (`KismetMathLibrary.MakeRotator` 0.0 0.0 (+ _returnvalue_yaw_5 90.0))))
  (bind (_returnvalue_roll_12 _returnvalue_pitch_12 _returnvalue_yaw_12) (`KismetMathLibrary.BreakRotator` (`KismetMathLibrary.MakeRotator` 0.0 0.0 (+ _returnvalue_yaw_6 90.0))))
  ; Colision detection on key press using sphere trace
  (:`Pressed`
    (bind (_outhit _returnvalue_2) (`KismetSystemLibrary.SphereTraceSingle` :`Start` _returnvalue :`End` _returnvalue :`Radius` 200.0 :`TraceChannel` "TraceTypeQuery1" :`bIgnoreSelf` false))
    (if _returnvalue_2
      (bind (_bblockinghit _binitialoverlap _time _distance _location _impactpoint _normal _impactnormal _physmat _hitactor _hitcomponent) (`GameplayStatics.BreakHitResult` _outhit))
      ; Branches comparing the detected object and calling the rotation code for the object
      (if (`ActorComponent.ComponentHasTag` _hitcomponent "Statue1")
        ; Takes the objects current rotation and location and rotates it 90 degrees in the z axis
        (`/Engine/EditorBlueprintResources/StandardMacros.DoOnce` false :!label _label
          (:`Completed`
            (`KismetSystemLibrary.MoveComponentTo` (`self.Statue1`) (`SceneComponent.RelativeLocation` _statue1) (`KismetMathLibrary.MakeRotator` 0.0 0.0 _returnvalue_yaw_7) false false 0.5)
            (`KismetSystemLibrary.Delay` 0.2)
            (goto _label :!via `Reset`)))
        (elif (`ActorComponent.ComponentHasTag` _hitcomponent "Statue2")
          ; Takes the objects current rotation and location and rotates it 90 degrees in the z axis
          (`/Engine/EditorBlueprintResources/StandardMacros.DoOnce` false :!label _label_2
            (:`Completed`
              (`KismetSystemLibrary.MoveComponentTo` (`self.Statue2`) (`SceneComponent.RelativeLocation` _statue2) (`KismetMathLibrary.MakeRotator` 0.0 0.0 _returnvalue_yaw_8) false false 0.5)
              (`KismetSystemLibrary.Delay` 0.2)
              (goto _label_2 :!via `Reset`)))
          (elif (`ActorComponent.ComponentHasTag` _hitcomponent "Statue3")
            ; Takes the objects current rotation and location and rotates it 90 degrees in the z axis
            (`/Engine/EditorBlueprintResources/StandardMacros.DoOnce` false :!label _label_3
              (:`Completed`
                (`KismetSystemLibrary.MoveComponentTo` (`self.Statue3`) (`SceneComponent.RelativeLocation` _statue3) (`KismetMathLibrary.MakeRotator` 0.0 0.0 _returnvalue_yaw_10) false false 0.5)
                (`KismetSystemLibrary.Delay` 0.2)
                (goto _label_3 :!via `Reset`)))
            (elif (`ActorComponent.ComponentHasTag` _hitcomponent "Statue4")
              ; Takes the objects current rotation and location and rotates it 90 degrees in the z axis
              (`/Engine/EditorBlueprintResources/StandardMacros.DoOnce` false :!label _label_4
                (:`Completed`
                  (`KismetSystemLibrary.MoveComponentTo` (`self.Statue4`) (`SceneComponent.RelativeLocation` _statue4) (`KismetMathLibrary.MakeRotator` 0.0 0.0 _returnvalue_yaw_11) false false 0.5)
                  (`KismetSystemLibrary.Delay` 0.2)
                  (goto _label_4 :!via `Reset`)))
              (elif (`ActorComponent.ComponentHasTag` _hitcomponent "Statue5")
                ; Takes the objects current rotation and location and rotates it 90 degrees in the z axis
                (`/Engine/EditorBlueprintResources/StandardMacros.DoOnce` false :!label _label_5
                  (:`Completed`
                    (`KismetSystemLibrary.MoveComponentTo` (`self.Statue5`) (`SceneComponent.RelativeLocation` _statue5) (`KismetMathLibrary.MakeRotator` 0.0 0.0 _returnvalue_yaw_12) false false 0.5)
                    (`KismetSystemLibrary.Delay` 0.2)
                    (goto _label_5 :!via `Reset`)))
                (elif (`ActorComponent.ComponentHasTag` _hitcomponent "Statue6")
                  ; Takes the objects current rotation and location and rotates it 90 degrees in the z axis
                  (`/Engine/EditorBlueprintResources/StandardMacros.DoOnce` false :!label _label_6
                    (:`Completed`
                      (`KismetSystemLibrary.MoveComponentTo` (`self.Statue6`) (`SceneComponent.RelativeLocation` _statue6) (`KismetMathLibrary.MakeRotator` 0.0 0.0 _returnvalue_yaw_9) false false 0.5)
                      (`KismetSystemLibrary.Delay` 0.2)
                      (goto _label_6 :!via `Reset`))))))))))))

(event `Key|E`
  (params (Key :type "Key Structure"))
  (bind _returnvalue (`SceneComponent.K2_GetComponentLocation` (`Character.CapsuleComponent` (`self.PlayerCharacter`))))
  ; Colision detection on key press using sphere trace
  (:`Pressed`
    (bind (_outhit _returnvalue_2) (`KismetSystemLibrary.SphereTraceSingle` :`Start` _returnvalue :`End` _returnvalue :`Radius` 200.0 :`TraceChannel` "TraceTypeQuery1" :`bIgnoreSelf` false))
    ; Checks to see if the colided object is the lever
    (if _returnvalue_2
      (if (`ActorComponent.ComponentHasTag` (`.HitComponent` (`GameplayStatics.BreakHitResult` _outhit)) "lever")
        ; Creates a timeline for the lever animation with max and min lever rotation in the lerp. The relative rotation is then passed the lerp. Finally, the function check statue is called.
        (bind (_direction _move) (`Timeline|Timeline` :!via `PlayFromStart`)
          (:`Update`
            (`SceneComponent.K2_SetRelativeRotation` (`self.Lever`) (`KismetMathLibrary.RLerp` (struct :`Pitch` 30.0) (struct :`Pitch` -40.0) _move) false false)
            (`self.CheckStatue`)))))))

(event `CheckStatue`
  (bind _door (`self.Door`))
  (bind _waterfall2 (`self.Waterfall2`))
  (bind _waterfall1 (`self.Waterfall1`))
  (bind _value (break `RigVMFunction_MathIntMake` (`self.PuzzleCompletion`)))
  (bind (_returnvalue_roll _returnvalue_pitch _returnvalue_yaw) (`KismetMathLibrary.BreakRotator` (`SceneComponent.K2_GetComponentRotation` (`self.Statue2`))))
  (bind (_returnvalue_roll_2 _returnvalue_pitch_2 _returnvalue_yaw_2) (`KismetMathLibrary.BreakRotator` (`SceneComponent.K2_GetComponentRotation` (`self.Statue4`))))
  (bind (_returnvalue_roll_3 _returnvalue_pitch_3 _returnvalue_yaw_3) (`KismetMathLibrary.BreakRotator` (`SceneComponent.K2_GetComponentRotation` (`self.Statue1`))))
  (bind (_returnvalue_roll_4 _returnvalue_pitch_4 _returnvalue_yaw_4) (`KismetMathLibrary.BreakRotator` (`SceneComponent.K2_GetComponentRotation` (`self.Statue2`))))
  (bind (_returnvalue_roll_5 _returnvalue_pitch_5 _returnvalue_yaw_5) (`KismetMathLibrary.BreakRotator` (`SceneComponent.K2_GetComponentRotation` (`self.Statue3`))))
  (bind (_returnvalue_roll_6 _returnvalue_pitch_6 _returnvalue_yaw_6) (`KismetMathLibrary.BreakRotator` (`SceneComponent.K2_GetComponentRotation` (`self.Statue5`))))
  (bind (_returnvalue_x _returnvalue_y _returnvalue_z) (`KismetMathLibrary.BreakVector` (`SceneComponent.K2_GetComponentLocation` _waterfall1)))
  (bind (_returnvalue_roll_7 _returnvalue_pitch_7 _returnvalue_yaw_7) (`KismetMathLibrary.BreakRotator` (`SceneComponent.K2_GetComponentRotation` (`self.Statue5`))))
  (bind (_returnvalue_roll_8 _returnvalue_pitch_8 _returnvalue_yaw_8) (`KismetMathLibrary.BreakRotator` (`SceneComponent.K2_GetComponentRotation` (`self.Statue4`))))
  (bind (_returnvalue_roll_9 _returnvalue_pitch_9 _returnvalue_yaw_9) (`KismetMathLibrary.BreakRotator` (`SceneComponent.K2_GetComponentRotation` (`self.Statue1`))))
  (bind (_returnvalue_roll_10 _returnvalue_pitch_10 _returnvalue_yaw_10) (`KismetMathLibrary.BreakRotator` (`SceneComponent.K2_GetComponentRotation` (`self.Statue6`))))
  (bind (_returnvalue_roll_11 _returnvalue_pitch_11 _returnvalue_yaw_11) (`KismetMathLibrary.BreakRotator` (`SceneComponent.K2_GetComponentRotation` (`self.Statue3`))))
  (bind (_returnvalue_x_2 _returnvalue_y_2 _returnvalue_z_2) (`KismetMathLibrary.BreakVector` (`SceneComponent.K2_GetComponentLocation` _door)))
  (bind (_returnvalue_roll_12 _returnvalue_pitch_12 _returnvalue_yaw_12) (`KismetMathLibrary.BreakRotator` (`SceneComponent.K2_GetComponentRotation` (`self.Statue4`))))
  (bind (_returnvalue_roll_13 _returnvalue_pitch_13 _returnvalue_yaw_13) (`KismetMathLibrary.BreakRotator` (`SceneComponent.K2_GetComponentRotation` (`self.Statue1`))))
  (bind (_returnvalue_roll_14 _returnvalue_pitch_14 _returnvalue_yaw_14) (`KismetMathLibrary.BreakRotator` (`SceneComponent.K2_GetComponentRotation` (`self.Statue2`))))
  (bind (_returnvalue_roll_15 _returnvalue_pitch_15 _returnvalue_yaw_15) (`KismetMathLibrary.BreakRotator` (`SceneComponent.K2_GetComponentRotation` (`self.Statue3`))))
  (bind (_returnvalue_x_3 _returnvalue_y_3 _returnvalue_z_3) (`KismetMathLibrary.BreakVector` (`SceneComponent.K2_GetComponentLocation` _waterfall2)))
  ; Puzzle completion is compaired to see what phase of the puzzle is being checked and will then run the current check values
  (if (>= _value 2)
    ; Checks that each statue rotation is true
    (if (== _returnvalue_yaw_10 -90.0)
      (if (== _returnvalue_yaw_7 90.0)
        (if (== _returnvalue_yaw_9 -90.0)
          (if (== _returnvalue_yaw -90.0)
            (if (== _returnvalue_yaw_11 90.0)
              (if (== _returnvalue_yaw_8 90.0)
                ; retrieves the current location and relative rotation and then moves the final door out of the level
                (`/Engine/EditorBlueprintResources/StandardMacros.DoOnce` false
                  (:`Completed`
                    (`KismetSystemLibrary.MoveComponentTo` (`self.Door`) (`KismetMathLibrary.MakeVector` _returnvalue_x_2 _returnvalue_y_2 (- _returnvalue_z_2 800.0)) (`SceneComponent.RelativeRotation` _door) false false 0.5)))))))))
    (elif (== _value 1)
      ; Checks that each statue rotation is true
      (if (== _returnvalue_yaw_6 180.0)
        (if (== _returnvalue_yaw_3 0.0)
          (if (== _returnvalue_yaw_4 180.0)
            (if (== _returnvalue_yaw_5 0.0)
              (if (== _returnvalue_yaw_2 180.0)
                ; retrieves the current location and relative rotation and then moves the waterfall out of the level
                (`/Engine/EditorBlueprintResources/StandardMacros.DoOnce` false
                  (:`Completed`
                    (`KismetSystemLibrary.MoveComponentTo` (`self.Waterfall1`) (`KismetMathLibrary.MakeVector` _returnvalue_x _returnvalue_y (* _returnvalue_z -2.0)) (`SceneComponent.RelativeRotation` _waterfall1) false false 0.5)
                    (set `self.PuzzleCompletion` (make `RigVMFunction_MathIntMake` 2)))))))))
      (elif (<= _value 0)
        ; Checks that each statue rotation is true
        (if (== _returnvalue_yaw_13 180.0)
          (if (== _returnvalue_yaw_14 -90.0)
            (if (== _returnvalue_yaw_15 0.0)
              (if (== _returnvalue_yaw_12 90.0)
                ; retrieves the current location and relative rotation and then moves the waterfall out of the level
                (`/Engine/EditorBlueprintResources/StandardMacros.DoOnce` false
                  (:`Completed`
                    (`KismetSystemLibrary.MoveComponentTo` (`self.Waterfall2`) (`KismetMathLibrary.MakeVector` _returnvalue_x_3 _returnvalue_y_3 (* _returnvalue_z_3 -2.0)) (`SceneComponent.RelativeRotation` _waterfall2) false false 0.5)
                    (set `self.PuzzleCompletion` (make `RigVMFunction_MathIntMake` 1)) ; Sets the puzzle completion value to be for the next phase
                  ))))))))))

(fn `UserConstructionScript`)